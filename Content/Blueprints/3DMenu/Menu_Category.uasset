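; Clickable category item in a 3D menu, spawned by a Mother actor for one of Housing, Business, Entertainment or Government.
; On BeginPlay it switches on its Category and adds a static mesh component for that category at runtime.
; Clicking the actor fires Selected, which reports the category back through Mother's SelectCategory.
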(event Custom|Selected
  ;[1 1 1] Tell mother to select my category
  (Default|SelectCategory (Variables|Default|GetMother) (Variables|Default|GetCategory)))

(event EventBeginPlay
  (bind _returnvalue (Math|Transform|MakeTransform "0, 0, 0" "0.000000,90.000000, 0" "1,1.000000,1"))
  ;[1 1 1] Begin play, get category based on mother spawning me and spawn a mesh
  (switch Utilities|FlowControl|Switch|SwitchonBuildingCategoriesEnum (Variables|Default|GetCategory)
    (:NewEnumerator0
      (AddComponent|AddStaticMeshComponent false _returnvalue))
    (:NewEnumerator1
      (AddComponent|AddStaticMeshComponent false _returnvalue))
    (:NewEnumerator2
      (AddComponent|AddStaticMeshComponent false _returnvalue))
    (:NewEnumerator3
      (AddComponent|AddStaticMeshComponent false _returnvalue))))

(event MouseInput|EventActorOnClicked
  (params (ButtonPressed :type Key%20Structure :default "AnyKey"))
  ;[1 1 1] Selected
  (CallFunction|Selected))

(fn ConstructionScript)