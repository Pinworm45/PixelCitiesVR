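; 3D building menu actor that shows category choices and housing options as child actors placed at arrow components.
; SpawnCategories creates Housing, Business, Entertainment and Government items, each holding a back-reference to the menu.
; SelectCategory clears them and, for Housing only, spawns six buildings at the first arrow, each assigned an arrow index to interpolate toward.
; CloseMenu destroys all tracked items; Tick is empty, with player-follow logic left disconnected.
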(event Custom|Spawn%20Categories
  (bind _categories (Variables|Default|GetCategories))
  ;[1 1 1] Spawn Categories
  (for (_array_element _array_index) (Variables|Default|GetArrowLocations)
    (switch int _array_index
      (:0
        (bind _returnvalue (AddComponent|AddChildActorComponent false (Transformation|GetRelativeTransform _array_element)))
        (bind _asmenu_category (Utilities|Casting|CastToMenu_Category (Variables|/Script/Engine.ChildActorComponent|GetChildActor _returnvalue)))
        (Variables|/Game/Blueprints/3DMenu/Menu_Category.Menu_Category_C|SetCategory _asmenu_category "NewEnumerator0")
        (Variables|/Game/Blueprints/3DMenu/Menu_Category.Menu_Category_C|SetMother _asmenu_category self)
        (Utilities|Array|Add _categories _asmenu_category))
      (:1
        (bind _returnvalue_2 (AddComponent|AddChildActorComponent false (Transformation|GetRelativeTransform _array_element)))
        (bind _asmenu_category_2 (Utilities|Casting|CastToMenu_Category (Variables|/Script/Engine.ChildActorComponent|GetChildActor _returnvalue_2)))
        (Variables|/Game/Blueprints/3DMenu/Menu_Category.Menu_Category_C|SetCategory _asmenu_category_2 "NewEnumerator1")
        (Variables|/Game/Blueprints/3DMenu/Menu_Category.Menu_Category_C|SetMother _asmenu_category_2 self)
        (Utilities|Array|Add _categories _asmenu_category_2))
      (:2
        (bind _returnvalue_3 (AddComponent|AddChildActorComponent false (Transformation|GetRelativeTransform _array_element)))
        (bind _asmenu_category_3 (Utilities|Casting|CastToMenu_Category (Variables|/Script/Engine.ChildActorComponent|GetChildActor _returnvalue_3)))
        (Variables|/Game/Blueprints/3DMenu/Menu_Category.Menu_Category_C|SetCategory _asmenu_category_3 "NewEnumerator2")
        (Variables|/Game/Blueprints/3DMenu/Menu_Category.Menu_Category_C|SetMother _asmenu_category_3 self)
        (Utilities|Array|Add _categories _asmenu_category_3))
      (:3
        (bind _returnvalue_4 (AddComponent|AddChildActorComponent false (Transformation|GetRelativeTransform _array_element)))
        (bind _asmenu_category_4 (Utilities|Casting|CastToMenu_Category (Variables|/Script/Engine.ChildActorComponent|GetChildActor _returnvalue_4)))
        (Variables|/Game/Blueprints/3DMenu/Menu_Category.Menu_Category_C|SetCategory _asmenu_category_4 "NewEnumerator3")
        (Variables|/Game/Blueprints/3DMenu/Menu_Category.Menu_Category_C|SetMother _asmenu_category_4 self)
        (Utilities|Array|Add _categories _asmenu_category_4)))))

(event Custom|SelectCategory
  (params (CategorySelected :type BuildingCategoriesEnum%20Enum))
  ;[1 1 1] Select Category
  (CallFunction|DespawnCategories)
  (switch Utilities|FlowControl|Switch|SwitchonBuildingCategoriesEnum CategorySelected
    (:NewEnumerator0
      (CallFunction|SpawnHousing))))

(event Custom|CloseMenu
  ;[1 1 1] Close Menu
  (CallFunction|DespawnCategories)
  (CallFunction|DespawnMenuBuildings))

(event Custom|DespawnMenuBuildings
  ;[1 1 1] Despawn Menu Buildings
  (for _array_element (Variables|Default|GetMenuBuildings)
    (Utilities|IsValid _array_element
      (:Is%20Valid
        (Actor|DestroyActor _array_element)))))

(event Custom|SpawnHousing
  (bind _category1arrow (Variables|Default|GetCategory1Arrow))
  (bind _returnvalue (Transformation|GetRelativeTransform _category1arrow))
  ;[1 1 1] Spawn Housing
  (Utilities|FlowControl|Sequence
    (:then_0
      (bind _returnvalue_2 (AddComponent|AddChildActorComponent false _returnvalue))
      (bind _asmenu_building (Utilities|Casting|CastToMenu_Building (Variables|/Script/Engine.ChildActorComponent|GetChildActor _returnvalue_2)))
      (Variables|/Game/Blueprints/3DMenu/Menu_Building.Menu_Building_C|SetHouseCategory _asmenu_building "NewEnumerator0")
      (Variables|/Game/Blueprints/3DMenu/Menu_Building.Menu_Building_C|SetMother _asmenu_building self)
      (Variables|/Game/Blueprints/3DMenu/Menu_Building.Menu_Building_C|SetArrowToInterpTo _asmenu_building 0)
      (Utilities|Array|Add (Variables|Default|GetMenuBuildings) _asmenu_building)
      (Variables|/Game/Blueprints/3DMenu/Menu_Building.Menu_Building_C|SetCategory _asmenu_building "NewEnumerator0"))
    (:then_1
      (bind _returnvalue_3 (AddComponent|AddChildActorComponent false _returnvalue))
      (bind _asmenu_building_2 (Utilities|Casting|CastToMenu_Building (Variables|/Script/Engine.ChildActorComponent|GetChildActor _returnvalue_3)))
      (Variables|/Game/Blueprints/3DMenu/Menu_Building.Menu_Building_C|SetHouseCategory _asmenu_building_2 "NewEnumerator4")
      (Variables|/Game/Blueprints/3DMenu/Menu_Building.Menu_Building_C|SetMother _asmenu_building_2 self)
      (Variables|/Game/Blueprints/3DMenu/Menu_Building.Menu_Building_C|SetArrowToInterpTo _asmenu_building_2 1)
      (Utilities|Array|Add (Variables|Default|GetMenuBuildings) _asmenu_building_2)
      (Variables|/Game/Blueprints/3DMenu/Menu_Building.Menu_Building_C|SetCategory _asmenu_building_2 "NewEnumerator0"))
    (:then_2
      (bind _returnvalue_4 (AddComponent|AddChildActorComponent false _returnvalue))
      (bind _asmenu_building_3 (Utilities|Casting|CastToMenu_Building (Variables|/Script/Engine.ChildActorComponent|GetChildActor _returnvalue_4)))
      (Variables|/Game/Blueprints/3DMenu/Menu_Building.Menu_Building_C|SetHouseCategory _asmenu_building_3 "NewEnumerator5")
      (Variables|/Game/Blueprints/3DMenu/Menu_Building.Menu_Building_C|SetMother _asmenu_building_3 self)
      (Variables|/Game/Blueprints/3DMenu/Menu_Building.Menu_Building_C|SetArrowToInterpTo _asmenu_building_3 2)
      (Utilities|Array|Add (Variables|Default|GetMenuBuildings) _asmenu_building_3)
      (Variables|/Game/Blueprints/3DMenu/Menu_Building.Menu_Building_C|SetCategory _asmenu_building_3 "NewEnumerator0"))
    (:then_3
      (bind _returnvalue_5 (AddComponent|AddChildActorComponent false _returnvalue))
      (bind _asmenu_building_4 (Utilities|Casting|CastToMenu_Building (Variables|/Script/Engine.ChildActorComponent|GetChildActor _returnvalue_5)))
      (Variables|/Game/Blueprints/3DMenu/Menu_Building.Menu_Building_C|SetHouseCategory _asmenu_building_4 "NewEnumerator1")
      (Variables|/Game/Blueprints/3DMenu/Menu_Building.Menu_Building_C|SetMother _asmenu_building_4 self)
      (Variables|/Game/Blueprints/3DMenu/Menu_Building.Menu_Building_C|SetArrowToInterpTo _asmenu_building_4 3)
      (Utilities|Array|Add (Variables|Default|GetMenuBuildings) _asmenu_building_4)
      (Variables|/Game/Blueprints/3DMenu/Menu_Building.Menu_Building_C|SetCategory _asmenu_building_4 "NewEnumerator0"))
    (:then_4
      (bind _returnvalue_6 (AddComponent|AddChildActorComponent false _returnvalue))
      (bind _asmenu_building_5 (Utilities|Casting|CastToMenu_Building (Variables|/Script/Engine.ChildActorComponent|GetChildActor _returnvalue_6)))
      (Variables|/Game/Blueprints/3DMenu/Menu_Building.Menu_Building_C|SetHouseCategory _asmenu_building_5 "NewEnumerator3")
      (Variables|/Game/Blueprints/3DMenu/Menu_Building.Menu_Building_C|SetMother _asmenu_building_5 self)
      (Variables|/Game/Blueprints/3DMenu/Menu_Building.Menu_Building_C|SetArrowToInterpTo _asmenu_building_5 4)
      (Utilities|Array|Add (Variables|Default|GetMenuBuildings) _asmenu_building_5)
      (Variables|/Game/Blueprints/3DMenu/Menu_Building.Menu_Building_C|SetCategory _asmenu_building_5 "NewEnumerator0"))
    (:then_5
      (bind _returnvalue_7 (AddComponent|AddChildActorComponent false _returnvalue))
      (bind _asmenu_building_6 (Utilities|Casting|CastToMenu_Building (Variables|/Script/Engine.ChildActorComponent|GetChildActor _returnvalue_7)))
      (Variables|/Game/Blueprints/3DMenu/Menu_Building.Menu_Building_C|SetHouseCategory _asmenu_building_6 "NewEnumerator2")
      (Variables|/Game/Blueprints/3DMenu/Menu_Building.Menu_Building_C|SetMother _asmenu_building_6 self)
      (Variables|/Game/Blueprints/3DMenu/Menu_Building.Menu_Building_C|SetArrowToInterpTo _asmenu_building_6 5)
      (Utilities|Array|Add (Variables|Default|GetMenuBuildings) _asmenu_building_6)
      (Variables|/Game/Blueprints/3DMenu/Menu_Building.Menu_Building_C|SetCategory _asmenu_building_6 "NewEnumerator0"))))

(event Custom|DespawnCategories
  ;[1 1 1] Despawn Categories
  (for _array_element (Variables|Default|GetCategories)
    (Utilities|IsValid _array_element
      (:Is%20Valid
        (Actor|DestroyActor _array_element)))))

(event EventTick
  (params (DeltaSeconds :type Float%20%28single-precision%29))
  ;[1 1 1] Tick / set location
)

(event EventBeginPlay
  ;[1 1 1] Begin play, spawn categories
  (Variables|Default|SetArrowLocations (Utilities|Array|MakeArray (Variables|Default|GetCategory1Arrow) (Variables|Default|GetCategory2Arrow) (Variables|Default|GetCategory3Arrow) (Variables|Default|GetCategory4Arrow) (Variables|Default|GetCategory5Arrow) (Variables|Default|GetCategory6Arrow))))

(fn ConstructionScript)

(fn SelectCategory)