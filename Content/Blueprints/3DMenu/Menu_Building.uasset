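; Clickable building item in the 3D build menu, representing one building the player can construct.
; On BeginPlay it adds a static mesh component chosen by its housing Category.
; Each Tick it eases toward its assigned arrow location on the Mother object using VInterpTo.
; Clicking it toggles the menu on the Governer pawn and tells that pawn to build BuildingToBuild.
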(event EventBeginPlay
  (bind _returnvalue (Math|Transform|MakeTransform "0, 0, 0" "0,90.000000, 0"))
  ;[1 1 1] Begin play, get category based on mother spawning me and spawn a mesh
  (switch Utilities|FlowControl|Switch|SwitchonHousingTypesEnum (Variables|Default|GetCategory)
    (:NewEnumerator0
      (AddComponent|AddStaticMeshComponent false _returnvalue))
    (:NewEnumerator3
      (AddComponent|AddStaticMeshComponent false _returnvalue))
    (:NewEnumerator2
      (AddComponent|AddStaticMeshComponent false _returnvalue))
    (:NewEnumerator1
      (AddComponent|AddStaticMeshComponent false _returnvalue))))

(event EventTick
  (params (DeltaSeconds :type Float%20%28single-precision%29))
  ;[1 1 1] Interp To Arrow Spot
  (Transformation|SetActorLocation (Math|Interpolation|VInterpTo (Transformation|GetActorLocation) (Transformation|GetWorldLocation (Utilities|Array|Get(acopy) (Variables|/Game/Blueprints/3DMenu/3DMenu.3DMenu_C|GetArrowLocations (Variables|Default|GetMother)) (Variables|Default|GetArrowToInterpTo))) DeltaSeconds 1.0) false false))

(event MouseInput|EventActorOnClicked
  (params (ButtonPressed :type Key%20Structure :default "AnyKey"))
  ;[1 1 1] On clicked tell governer to build BuildingToMake
  (bind _asbp_governer_pawn (Utilities|Casting|CastToBP_Governer_Pawn (Game|Player|GetPlayerPawn 0)))
  (Default|ToggleMenu _asbp_governer_pawn)
  (Default|Build _asbp_governer_pawn (Variables|Default|GetBuildingToBuild)))

(fn ConstructionScript)