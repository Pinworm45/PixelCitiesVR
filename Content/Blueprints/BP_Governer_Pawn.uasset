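; Player pawn for a building game, providing a 3D in-world menu for choosing buildings to place, with VR and mouse support.
; While the menu is open, a gated Tick spins the hovered category or building, found by camera trace with an HMD or cursor trace otherwise.
; Gamepad accept always camera-traces, then opens the category or starts build mode and toggles the menu.
; It also creates the settings menu and forwards input to ActionManager for keybinding.
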(event MenuPressed(ActionManager)
  (bind _settingsmenu (Variables|Default|GetSettingsMenu))
  ;[1 1 1] Open/Close Menu
  (if (Variables|/Game/QualityMenu/HUD_UMG_Classic/ClassicSettingsMain.ClassicSettingsMain_C|GetIs%20Menu%20Open _settingsmenu)
    (Default|CloseMenu _settingsmenu)
    (else
      (Default|OpenMenu _settingsmenu))))

(event MoveForward(ActionManager)
  (params (Axis :type Float%20%28single-precision%29))
  ;[1 1 1] Movement
  (if (!= Axis 0.0)
    _))

(event Custom|Build
  (params (BuildingToMake :type Base%20Building%20Class%20Reference))
  ;[1 1 1] Build
  (Class|GovernerPawn|SelectedforPlacement BuildingToMake)
  (Utilities|FlowControl|Delay 0.15)
  (bind _asgoverner_pawn (Utilities|Casting|CastToGovernerPawn (Game|Player|GetPlayerPawn 0)))
  (Variables|/Script/PixelCitiesVR.GovernerPawn|SetbBuildMode _asgoverner_pawn true))

(event Custom|DisableMenuTrace
  (bind _returnvalue (Game|GetPlayerController 0))
  (bind _hitresult (Game|Player|GetHitResultUnderCursorbyChannel _returnvalue "TraceTypeQuery1" true))
  (bind _hitactor (Collision|BreakHitResult _hitresult))
  ;[1 1 1] Tick / menu trace
  (Utilities|FlowControl|Gate true) ; enters at Close
)

(event Custom|EnableMenuTrace
  (bind _returnvalue (Game|GetPlayerController 0))
  (bind _hitresult (Game|Player|GetHitResultUnderCursorbyChannel _returnvalue "TraceTypeQuery1" true))
  (bind _hitactor (Collision|BreakHitResult _hitresult))
  ;[1 1 1] Tick / menu trace
  (Utilities|FlowControl|Gate true) ; enters at Open
)

(event EventTick
  (params (DeltaSeconds :type Float%20%28single-precision%29))
  (bind _returnvalue (Game|GetPlayerController 0))
  (bind _hitresult (Game|Player|GetHitResultUnderCursorbyChannel _returnvalue "TraceTypeQuery1" true))
  (bind _hitactor (Collision|BreakHitResult _hitresult))
  ;[1 1 1] Tick / menu trace
  (Utilities|FlowControl|Gate true
    (:Exit
      ;[1 1 1] Check for HMD
      (if (Class|HeadMountedDisplayFunctionLibrary|IsHeadMountedDisplayEnabled)
        ;[1 1 1] If HMD do linetrace
        (bind _outhit (CallFunction|LineTraceforMenu 5e+03))
        (bind _asmenu_category (Utilities|Casting|CastToMenu_Category (.HitActor (Collision|BreakHitResult _outhit)))
          (:then
            (Transformation|AddActorLocalRotation _asmenu_category "0,1.500000, 0" false false))
          (:CastFailed
            (bind _asmenu_building (Utilities|Casting|CastToMenu_Building (.HitActor (Collision|BreakHitResult _outhit))))
            (Transformation|AddActorLocalRotation _asmenu_building "0,1.500000, 0" false false)))
        (else
          ;[1 1 1] if no HMD get results under cursor
          (bind _asmenu_category_2 (Utilities|Casting|CastToMenu_Category _hitactor)
            (:then
              (Transformation|AddActorLocalRotation _asmenu_category_2 "0,1.500000, 0" false false))
            (:CastFailed
              (bind _asmenu_building_2 (Utilities|Casting|CastToMenu_Building _hitactor))
              (Transformation|AddActorLocalRotation _asmenu_building_2 "0,1.500000, 0" false false))))))))

(event EventBeginPlay
  (bind _returnvalue (Game|GetPlayerController 0))
  ;[1 1 1] Begin play, set vars, enable mouse stuff on PC
  (bind _as3dmenu (Utilities|Casting|CastTo3DMenu (Variables|/Script/Engine.ChildActorComponent|GetChildActor (Variables|Default|Get3DMenu))))
  (Variables|Default|Set3DMenuGUI _as3dmenu)
  (Variables|/Script/Engine.PlayerController|SetbEnableMouseOverEvents _returnvalue true)
  (Variables|/Script/Engine.PlayerController|SetbEnableClickEvents _returnvalue true)
  (Variables|/Script/Engine.PlayerController|SetbShowMouseCursor _returnvalue true)
  ;[1 1 1] Set up Quality Menu
  (bind _game_settings (Utilities|GetGameSettings (Game|GetGameInstance)))
  (Variables|Default|SetGameSettings _game_settings)
  (bind _returnvalue_2 (UserInterface|CreateWidget "/Game/QualityMenu/HUD_UMG_Classic/ClassicSettingsMain.ClassicSettingsMain_C" 0 true true (Variables|Default|GetActionManager)))
  (bind _output_get (Variables|Default|SetSettingsMenu _returnvalue_2))
  (UserInterface|Viewport|AddtoViewport _output_get 1)
  (Utilities|AddCameraFieldOfViewControl (Variables|Default|GetCamera) (Game|GetGameInstance)))

(event Input|AxisEvents|InputAxisUpdateKeybinding
  (params (AxisValue :type Float%20%28single-precision%29))
  ;[1 1 1] Update Keybindings
  (Default|TickActionManager (Variables|Default|GetActionManager)))

(event Input|KeyboardEvents|F
  (params (Key :type Key%20Structure :default "AnyKey"))
  ;[1 1 1] F to toggle menu
  (:Pressed
    (CallFunction|ToggleMenu)))

(event Input|GamepadEvents|GamepadFaceButtonLeft
  (params (Key :type Key%20Structure :default "AnyKey"))
  ;[1 1 1] F to toggle menu
  (:Pressed
    (CallFunction|ToggleMenu)))

(event Input|KeyboardEvents|AnyKey
  (params (Key :type Key%20Structure :default "AnyKey"))
  ;[1 1 1] Update Keybindings
  (:Pressed
    (Default|AnyKeyPress (Variables|Default|GetActionManager) (Utilities|Struct|MakeKeyInput Key false))))

(event Input|GamepadEvents|GamepadFaceButtonBottom
  (params (Key :type Key%20Structure :default "AnyKey"))
  ;[1 1 1] Accept Button / select category / building
  (:Pressed
    (bind _outhit (CallFunction|LineTraceforMenu 4e+03))
    (bind _asmenu_category (Utilities|Casting|CastToMenu_Category (.HitActor (Collision|BreakHitResult _outhit)))
      (:then
        (Default|SelectCategory (Variables|Default|Get3DMenuGUI) (Variables|/Game/Blueprints/3DMenu/Menu_Category.Menu_Category_C|GetCategory _asmenu_category)))
      (:CastFailed
        (bind _asmenu_building (Utilities|Casting|CastToMenu_Building (.HitActor (Collision|BreakHitResult _outhit))))
        (CallFunction|Build (Variables|/Game/Blueprints/3DMenu/Menu_Building.Menu_Building_C|GetBuildingToBuild _asmenu_building))
        (CallFunction|ToggleMenu)))))

(fn ConstructionScript)

(fn ToggleMenu
  (if (Variables|Default|GetMenuIsOpen?)
    (Variables|Default|SetMenuIsOpen? false)
    (Default|CloseMenu (Variables|Default|Get3DMenuGUI))
    (CallFunction|DisableMenuTrace)
    (else
      (Variables|Default|SetMenuIsOpen? true)
      (Default|SpawnCategories (Variables|Default|Get3DMenuGUI))
      (CallFunction|EnableMenuTrace))))

(fn LineTraceforMenu
  (params (Distance :type Float%20%28single-precision%29))
  (bind _returnvalue (Game|GetPlayerCameraManager 0))
  (bind _returnvalue_2 (Transformation|GetActorLocation _returnvalue))
  (bind _outhit (Collision|LineTraceByChannel _returnvalue_2 (+ _returnvalue_2 (* (Transformation|GetActorForwardVector _returnvalue) Distance)) "TraceTypeQuery1" false 0 "None"))
  (return _outhit))