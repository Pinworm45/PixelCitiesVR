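; BP_KeyInput wraps a single key binding for the keybinding system and reports its axis value, down, just-pressed and just-released state from a player controller.
; Init remaps the key through ReplaceKeyMapping, which also selects whether an analog axis reads its negative or positive half.
; Float axes act as buttons at a fixed threshold, with edges detected against a cached previous value.
; SaveKeyInput stores the binding in GameSettings.
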(fn InitKeyInput
  (params (Key%20Input :type Key%20Input%20Structure))
  (bind _returnvalue (Utilities|ReplaceKeyMapping Key%20Input))
  (bind (_input _usenegativeaxis) (Utilities|Struct|BreakKeyInput _returnvalue))
  (Variables|Default|SetKey%20Input _input)
  (Variables|Default|SetAnalog%20Use%20Negative%20Axis _usenegativeaxis)
  (return self))

(fn KeyInputCurrentState
  (params (Controller :type Player%20Controller%20Object%20Reference))
  (bind _key_input (Variables|Default|GetKey%20Input))
  (bind _key_input_2 (Variables|Default|GetKey%20Input))
  (bind _analog_use_negative_axis (Variables|Default|GetAnalog%20Use%20Negative%20Axis))
  (bind _analog_previous_axis_value (Variables|Default|GetAnalog%20Previous%20Axis%20Value))
  (bind _returnvalue (Game|Player|IsInputKeyDown Controller _key_input_2))
  (bind _returnvalue_2 (Class|PlayerController|GetInputAnalogKeyState Controller _key_input))
  (bind _returnvalue_3 (Math|Float|Min(Float) _returnvalue_2 0.0))
  (bind _returnvalue_4 (Math|Float|Max(Float) _returnvalue_2 0.0))
  (bind _returnvalue_5 (Math|Float|Absolute(Float) _returnvalue_3))
  (bind _returnvalue_6 (Math|Float|SelectFloat _returnvalue_5 _returnvalue_4 _analog_use_negative_axis))
  (Utilities|IsValid Controller
    (:Is%20Valid
      (if (Class|KismetInputLibrary|KeyIsFloatAxis _key_input_2)
        ;[1 1 1] Analog Axis Input
        (return _returnvalue_6 (>= _returnvalue_6 0.1) (and (>= _returnvalue_6 0.1) (< _analog_previous_axis_value 0.1)) (and (< _returnvalue_6 0.1) (>= _analog_previous_axis_value 0.1)))
        (else
          ;[1 1 1] Button Input
          (return (Math|Conversions|ToFloat(Boolean) _returnvalue) _returnvalue (Game|Player|WasInputKeyJustPressed Controller _key_input_2) (Class|PlayerController|WasInputKeyJustReleased Controller _key_input_2)))))
    (:Is%20Not%20Valid
      (Development|PrintString 0 (Utilities|String|Append "Err: BP_Keyinput, " (Utilities|String|ToString(Text) (Class|KismetInputLibrary|KeyGetDisplayName (Variables|Default|GetKey%20Input))) "Player Controller is not valid."))
      (return 0.0 false false false))))

(fn UpdatePreviousAnalogAxisValue
  (params (Player%20Controller :type Player%20Controller%20Object%20Reference))
  (bind _key_input (Variables|Default|GetKey%20Input))
  (bind _returnvalue (Class|PlayerController|GetInputAnalogKeyState Player%20Controller _key_input))
  (Variables|Default|SetAnalog%20Previous%20Axis%20Value (Variables|Default|GetAnalog%20Current%20Axis%20Value))
  (Variables|Default|SetAnalog%20Current%20Axis%20Value (Math|Float|SelectFloat (Math|Float|Absolute(Float) (Math|Float|Min(Float) _returnvalue 0.0)) (Math|Float|Max(Float) _returnvalue 0.0) (Variables|Default|GetAnalog%20Use%20Negative%20Axis))))

(fn SaveKeyInput
  (params (Game%20Settings :type Game%20Settings%20Object%20Reference) (ActionName :type String) (Category :type String) (Name :type String) (Scale :type Float%20%28single-precision%29) (Primary :type Boolean))
  (Default|StoreKeyInput Game%20Settings ActionName Category Name Scale Primary (Variables|Default|GetKey%20Input) (Variables|Default|GetAnalog%20Use%20Negative%20Axis) false))