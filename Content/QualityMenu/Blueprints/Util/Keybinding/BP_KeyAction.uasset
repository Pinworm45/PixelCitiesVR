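; BP_KeyAction is a named, categorized input action in the keybinding system, built from a set of BP_KeyMapping objects.
; Init constructs the mappings and warns about duplicate names; lookup by name ignores case.
; Per-player-controller state sums mapping values, reporting a press when all active mappings were just pressed and a release when none remain active after one was released.
; Save and load delegate to each mapping through GameSettings.
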(fn InitKeyAction
  (params (Key%20Action :type Key%20Action%20Structure) (Action%20Name :type String))
  (bind (_category _keymappings) (Utilities|Struct|BreakKeyAction Key%20Action))
  (bind _self self)
  (Variables|Default|SetAction%20Name Action%20Name)
  (Variables|Default|SetCategory _category)
  (for _array_element _keymappings
    (bind _returnvalue (Game|ConstructObjectfromClass "/Game/QualityMenu/Blueprints/Util/Keybinding/BP_KeyMapping.BP_KeyMapping_C" _self _self))
    (bind _mapping (Default|InitKeyMapping _returnvalue _array_element))
    (Utilities|Array|Add (Variables|Default|GetKey%20Mappings) _mapping)
    (|WarningIfDuplicateNamedMappings (.Name (Utilities|Struct|BreakKeyMapping _array_element))))
  (return self))

(fn KeyActionCurrentState
  (params (Player%20Controller :type Player%20Controller%20Object%20Reference))
  (bind _active_mappings (LocalVariables|GetActive%20Mappings))
  (for _array_element (Variables|Default|GetKey%20Mappings)
    (bind (_mapping_value _is_active _just_pressed _just_released) (Default|KeyMappingCurrentState _array_element Player%20Controller))
    (LocalVariables|SetAction%20Value (+ _mapping_value (LocalVariables|GetAction%20Value)))
    (Utilities|IncrementIntifTrue (LocalVariables|GetActive%20Mappings) _is_active
      (:%20%20
        (Utilities|IncrementIntifTrue (LocalVariables|GetTimes%20Just%20Pressed) _just_pressed
          (:%20%20
            (Utilities|IncrementIntifTrue (LocalVariables|GetTimes%20Just%20Released) _just_released))))))
  (return (LocalVariables|GetAction%20Value) (and (== (LocalVariables|GetTimes%20Just%20Pressed) _active_mappings) (> _active_mappings 0)) (and (== _active_mappings 0) (> (LocalVariables|GetTimes%20Just%20Released) 0))))

(fn SaveAction
  (params (Game%20Settings :type Game%20Settings%20Object%20Reference))
  (for _array_element (Variables|Default|GetKey%20Mappings)
    (Default|SaveKeyMapping _array_element Game%20Settings (Variables|Default|GetAction%20Name) (Variables|Default|GetCategory))))

(fn LoadAction
  (params (Game%20Settings :type Game%20Settings%20Object%20Reference))
  (for _array_element (Variables|Default|GetKey%20Mappings)
    (Default|LoadKeyMapping _array_element Game%20Settings (Variables|Default|GetAction%20Name) (Variables|Default|GetCategory))))

(fn GetMapping
  (params (Mapping%20Name :type String))
  (for _array_element (Variables|Default|GetKey%20Mappings)
    (if (Utilities|Enum|Equal(Enum) (Utilities|String|ToLower (Variables|/Game/QualityMenu/Blueprints/Util/Keybinding/BP_KeyMapping.BP_KeyMapping_C|GetName _array_element)) (Utilities|String|ToLower Mapping%20Name))
      (LocalVariables|SetResult _array_element)))
  (Utilities|IsValid (LocalVariables|GetResult)
    (:Is%20Valid
      _)
    (:Is%20Not%20Valid
      (Development|PrintString 0 (Utilities|String|Append "Err: BP_KeyAction " (Variables|Default|GetAction%20Name) " could not find mapping " Mapping%20Name))))
  (return (LocalVariables|GetResult) (Utilities|IsValid (LocalVariables|GetResult))))