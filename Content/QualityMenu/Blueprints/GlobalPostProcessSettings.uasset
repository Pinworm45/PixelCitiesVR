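; Quality Menu actor that applies the game settings' gamma, bloom and gain to a global PostProcess component.
; On BeginPlay it gets Game Settings from the GameInstance, registers itself as the global post process interface, then applies the values, or logs an error and deactivates the component on failure.
; When replaced by a different controller, it deactivates its post process and shows that on its TextRender.
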(event EventBeginPlay
  (bind _game_settings (Utilities|GetGameSettings (Game|GetGameInstance)))
  (bind _output_get (Variables|Default|SetGameSettings _game_settings))
  (Utilities|IsValid _output_get
    (:Is%20Valid
      (bind _replaced (Utilities|SetGlobalPostProcess (Game|GetGameInstance) self))
      (if _replaced
        (CallFunction|UpdateGlobalPostEffects)
        (else
          (Development|PrintString "Error: QualityMenu: GobalPostProcessSetting. Global Post Process setting controller exists in Game settings and did not want to be replaced.")
          (Components|Activation|Deactivate (Variables|Default|GetPostProcess) :!label _label))))
    (:Is%20Not%20Valid
      (Development|PrintString "Error: QualityMenu: GobalPostProcessSetting. Global Post Process setting could not get Game Settings from Game Instance. ")
      (goto _label))))

(fn ConstructionScript)

(fn UpdateGlobalPostEffects
  (bind _gamesettings (Variables|Default|GetGameSettings))
  (CallFunction|UpdateGamma (Default|GetGammaIntensity _gamesettings))
  (CallFunction|UpdateBloom (Default|GetBloomIntensity _gamesettings))
  (CallFunction|UpdateGain (Default|GetGainIntensity _gamesettings)))

(fn ReplaceGlobalPostProcess
  (params (New%20Global%20Post%20Process :type Global%20Post%20Process%20Interface%20Interface))
  (if (== (Utilities|ToObject(Interface) New%20Global%20Post%20Process) self) ; Do not replace post process if its the same
    _
    (else
      (Components|Activation|Deactivate (Variables|Default|GetPostProcess))
      (Rendering|Components|TextRender|SetText (Variables|Default|GetTextRender) (Utilities|Text|MakeLiteralText "Quality Menu 
Global Post Process 
Deactivated"))))
  (return true))

(fn UpdateBloom
  (params (Bloom%20Strength :type Float%20%28single-precision%29))
  (Utilities|Struct|SetmembersinPostProcessSettings (Variables|/Script/Engine.PostProcessComponent|GetSettings (Variables|Default|GetPostProcess)) Bloom%20Strength)
  (return false))

(fn UpdateGain
  (params (Gain%20Strength :type Float%20%28single-precision%29))
  (Utilities|Struct|SetmembersinPostProcessSettings (Variables|/Script/Engine.PostProcessComponent|GetSettings (Variables|Default|GetPostProcess)) (Math|Conversions|ToVector(Float) Gain%20Strength))
  (return false))

(fn UpdateGamma
  (params (Gamma%20Strength :type Float%20%28single-precision%29))
  (Utilities|Struct|SetmembersinPostProcessSettings (Variables|/Script/Engine.PostProcessComponent|GetSettings (Variables|Default|GetPostProcess)) (Math|Conversions|ToVector(Float) Gamma%20Strength))
  (return false))